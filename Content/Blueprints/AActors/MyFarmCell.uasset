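; MyFarmCell is a farm tile actor that highlights under the cursor and changes its look according to farming actions.
; Cursor hover events on CellMesh set the "light" material vector parameter to add or remove the highlight.
; The ModifyCell event forwards its message to ChangeCellMaterial, which swaps the mesh material for Harvest, Sow and Plow.
; Watering keeps the material and activates the Niagara effect, which this Blueprint never deactivates.
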(event `self.CellMesh.OnBeginCursorOver`
  (params (TouchedComponent :type "PrimitiveComponent Object Reference"))
  (`MeshComponent.SetVectorParameterValueOnMaterials` (`self.CellMesh`) "light" (0.1 0.1 0.1)))

(event `self.CellMesh.OnEndCursorOver`
  (params (TouchedComponent :type "PrimitiveComponent Object Reference"))
  (`MeshComponent.SetVectorParameterValueOnMaterials` (`self.CellMesh`) "light" (0.0 0.0 0.0)))

(event `self.ModifyCell`
  (params (Mensaje :type String))
  (`self.ChangeCellMaterial` Mensaje))

(fn `UserConstructionScript`)